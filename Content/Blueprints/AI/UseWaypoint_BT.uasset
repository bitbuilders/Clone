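; Behavior tree decorator that passes when the AI's controlled pawn is within a set Distance of the TargetLocation blackboard vector, likely gating waypoint use.
; It casts the owner to AIControllerFollow_BP on first use and caches the controller reference for later checks.
; The check compares the straight-line 3D length between pawn and target against Distance, inclusive.
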(fn PerformConditionCheck
  (params (OwnerActor :type Actor%20Object%20Reference))
  (if (!= (Variables|Default|GetAIControllerRef) 0)
    _
    (else
      (bind _asaicontroller_follow_bp (Utilities|Casting|CastToAIControllerFollow_BP OwnerActor))
      (Variables|Default|SetAIControllerRef _asaicontroller_follow_bp)))
  (return (<= (Math|Vector|VectorLength (- (Transformation|GetActorLocation (Pawn|GetControlledPawn (Variables|Default|GetAIControllerRef))) (Class|BTFunctionLibrary|GetBlackboardValueasVector (Variables|Default|GetTargetLocation)))) (Variables|Default|GetDistance))))