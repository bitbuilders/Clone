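; AI controller that starts the Logic_BT behavior tree on the Follow_BB blackboard for its pawn.
; On BeginPlay it seeds HomeLocation and TargetLocation with the pawn's position and caches every TargetPoint in Waypoints; the "Waypoint" tag check does not filter them.
; GetWaypoint writes a randomly chosen cached point to the Waypoint blackboard key.
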(event Custom|Get%20Waypoint
  (bind _waypoints (Variables|Default|GetWaypoints))
  (AI|Components|Blackboard|SetValueasObject (Variables|Default|GetBlackboard) (Utilities|Name|MakeLiteralName "Waypoint") (Utilities|Array|Get(acopy) _waypoints (Math|Random|RandomIntegerinRange 0 (- (Utilities|Array|Length _waypoints) 1)))))

(event EventBeginPlay
  (bind _blackboardcomponent (Class|AIController|UseBlackboard "/Game/Blueprints/AI/Follow_BB.Follow_BB"))
  (AI|Components|Blackboard|SetValueasVector _blackboardcomponent (Variables|Default|GetHomeLocation) (Transformation|GetActorLocation (Pawn|GetControlledPawn)))
  (AI|Components|Blackboard|SetValueasVector _blackboardcomponent (Variables|Default|GetTargetLocation) (Transformation|GetActorLocation (Pawn|GetControlledPawn)))
  (AI|RunBehaviorTree "/Game/Blueprints/AI/Logic_BT.Logic_BT")
  ;[1 1 1] Get Waypoints
  (bind _outactors (Actor|GetAllActorsOfClass "/Script/Engine.TargetPoint"))
  (bind _array_element (Utilities|Array|ForEachLoopwithBreak _outactors)
    (:LoopBody
      (if (Actor|ActorHasTag _array_element "Waypoint")
        _
        (else
          _))
      (Utilities|Array|Add (Variables|Default|GetWaypoints) _array_element))))

(event EventTick
  (params (DeltaSeconds :type Float%20%28single-precision%29)))

(fn ConstructionScript)