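; Behavior Tree task that picks a random waypoint for an AI run by AIControllerFollow_BP.
; On execute it caches the controller, then selects one of the first four TargetPoint actors found in the level.
; It stores that actor's location in the HomeLocation blackboard key, copies it to the TargetLocation key and finishes successfully.
; If the controller cast fails, the task never calls FinishExecute.
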(event EventReceiveExecute
  (params (OwnerActor :type Actor%20Object%20Reference))
  (if (!= (Variables|Default|GetAIControllerRef) 0)
    _
    (else
      (bind _asaicontroller_follow_bp (Utilities|Casting|CastToAIControllerFollow_BP OwnerActor))
      (Variables|Default|SetAIControllerRef _asaicontroller_follow_bp)))
  (bind _outactors (Actor|GetAllActorsOfClass "/Script/Engine.TargetPoint"))
  (AI|Components|Blackboard|SetValueasVector (AI|GetBlackboard (Variables|Default|GetAIControllerRef)) (Variables|Default|GetHomeLocation) (Transformation|GetActorLocation (Utilities|Array|Get(acopy) _outactors (Math|Random|RandomIntegerinRange 0 3))))
  (AI|BehaviorTree|SetBlackboardValueasVector (Variables|Default|GetTargetLocation) (AI|Components|Blackboard|GetValueasVector (AI|GetBlackboard (Variables|Default|GetAIControllerRef)) (Variables|Default|GetHomeLocation)))
  (AI|BehaviorTree|FinishExecute true))