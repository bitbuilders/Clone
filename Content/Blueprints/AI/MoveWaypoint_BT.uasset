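; Behavior tree task that moves the AI's controlled pawn to the actor stored in the Waypoint blackboard key.
; On execute it casts the owner to AIControllerFollow_BP and caches it for later runs, then calls AIMoveTo with a fixed acceptance radius.
; The task finishes successfully when the move succeeds; a failed move or failed cast never calls FinishExecute.
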(event EventReceiveExecute
  (params (OwnerActor :type Actor%20Object%20Reference))
  (if (!= (Variables|Default|GetAIControllerRef) 0)
    _
    (else
      (bind _asaicontroller_follow_bp (Utilities|Casting|CastToAIControllerFollow_BP OwnerActor))
      (Variables|Default|SetAIControllerRef _asaicontroller_follow_bp)))
  (AI|AIMoveTo (Pawn|GetControlledPawn (Variables|Default|GetAIControllerRef)) "0, 0, 0" (AI|BehaviorTree|GetBlackboardValueasActor (Variables|Default|GetWaypoint)) 1e+02 false
    (:OnSuccess
      (AI|BehaviorTree|FinishExecute true))))