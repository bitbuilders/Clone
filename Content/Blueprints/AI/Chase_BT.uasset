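; Behavior Tree task that sends the AI's controlled pawn chasing the actor stored in the TargetFollow blackboard key.
; The first execution caches the AIControllerFollow_BP owner, starts the move and calls Run on the AICharacter_BP pawn.
; Later executions reuse the cached controller and only issue AIMoveTo.
; The task finishes as successful whether the move succeeds or fails.
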(event EventReceiveExecute
  (params (OwnerActor :type Actor%20Object%20Reference))
  (if (!= (Variables|Default|GetAIControllerRef) 0)
    (AI|AIMoveTo (Pawn|GetControlledPawn (Variables|Default|GetAIControllerRef)) "0, 0, 0" (AI|BehaviorTree|GetBlackboardValueasActor (Variables|Default|GetTargetFollow)) 5.0 false :!label _label
      (:OnSuccess
        _)
      (:OnFail
        _))
    (AI|BehaviorTree|FinishExecute true)
    (else
      (bind _asaicontroller_follow_bp (Utilities|Casting|CastToAIControllerFollow_BP OwnerActor))
      (Variables|Default|SetAIControllerRef _asaicontroller_follow_bp)
      (Utilities|FlowControl|Sequence
        (:then_0
          (goto _label))
        (:then_1
          (bind _asaicharacter_bp (Utilities|Casting|CastToAICharacter_BP (Pawn|GetControlledPawn (Variables|Default|GetAIControllerRef))))
          (Default|Run _asaicharacter_bp))))))