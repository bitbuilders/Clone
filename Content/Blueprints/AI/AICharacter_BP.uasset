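; AI character Blueprint that takes damage from bullets and dies when its health runs out.
; Overlapping actors tagged "Bullet" subtract base damage, multiplied for powerful laser beams, and are then destroyed.
; A death or hit effect spawns at the bullet's location, with removal scripted after a short delay.
; AI perception updates only cast sensed actors to the first-person character; the "Caught!" print is disconnected.
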(event OnPerceptionUpdated(AIPerception)
  (params (UpdatedActors :type Array%20of%20Actor%20Object%20References))
  (bind _array_element (Utilities|Array|ForEachLoopwithBreak UpdatedActors)
    (:LoopBody
      (Utilities|Casting|CastToFirstPersonCharacter _array_element))))

(event Collision|EventActorBeginOverlap
  (params (OtherActor :type Actor%20Object%20Reference))
  (if (Actor|ActorHasTag OtherActor "Bullet")
    (Utilities|Casting|CastToLazerBeam_Powerful_BP OtherActor
      (:then
        (Variables|Default|SetHealth (- (Variables|Default|GetHealth) (* (Variables|Default|GetBulletBaseDamage) (Variables|Default|GetPowerfulBulletMultiplier)))))
      (:CastFailed
        (Variables|Default|SetHealth (- (Variables|Default|GetHealth) (Variables|Default|GetBulletBaseDamage)))))
    (Actor|DestroyActor OtherActor)
    (if (<= (Variables|Default|GetHealth) 0.0)
      (Actor|DestroyActor)
      (bind _returnvalue (Game|SpawnActorfromClass "/Game/Blueprints/DieEffect_BP.DieEffect_BP_C" (Math|Conversions|ToTransform(Vector) (Transformation|GetActorLocation OtherActor)) "Undefined" 0 0))
      (Utilities|FlowControl|Delay 2.0)
      (Actor|DestroyActor _returnvalue)
      (else
        (bind _returnvalue_2 (Game|SpawnActorfromClass "/Game/Blueprints/HitEffect.HitEffect_C" (Math|Conversions|ToTransform(Vector) (Transformation|GetActorLocation OtherActor)) "Undefined" 0 0))
        (Utilities|FlowControl|Delay 2.0)
        (Actor|DestroyActor _returnvalue_2)))))

(fn ConstructionScript)