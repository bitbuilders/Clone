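; Behavior tree service that detects targets in front of an AI pawn for following.
; Each tick it sphere-traces around the pawn for the desired object type, using a cached AIControllerFollow_BP and ignoring other AI characters.
; Each hit passing a line-of-sight trace and forward dot-product check sets TargetFollow and TargetLocation.
; Failing hits or empty results clear only TargetFollow, so the last hit evaluated decides the target.
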(event EventTick
  (params (OwnerActor :type Actor%20Object%20Reference) (DeltaSeconds :type Float%20%28single-precision%29))
  (bind _targetfollow (Variables|Default|GetTargetFollow))
  (Utilities|FlowControl|Sequence
    (:then_0
      (if (!= (Variables|Default|GetAIControllerRef) 0)
        _
        (else
          (bind _asaicontroller_follow_bp (Utilities|Casting|CastToAIControllerFollow_BP OwnerActor))
          (Variables|Default|SetAIControllerRef _asaicontroller_follow_bp)))
      (bind _outactors (Actor|GetAllActorsOfClass "/Game/Blueprints/AI/AICharacter_BP.AICharacter_BP_C"))
      (Variables|Default|SetLocation (Transformation|GetActorLocation (Pawn|GetControlledPawn (Variables|Default|GetAIControllerRef))))
      (bind _outhits (Collision|MultiSphereTraceForObjects (Transformation|GetActorLocation (Pawn|GetControlledPawn (Variables|Default|GetAIControllerRef))) (+ (Transformation|GetActorLocation (Pawn|GetControlledPawn (Variables|Default|GetAIControllerRef))) "0, 0,10.000000") 3e+03 (Utilities|Array|MakeArray (Variables|Default|GetDesiredObjectType)) false _outactors "None"))
      (if (> (Utilities|Array|Length _outhits) 0)
        (bind _array_element (Utilities|Array|ForEachLoopwithBreak _outhits)
          (:LoopBody
            (bind _outhit (Collision|LineTraceByChannel (Variables|Default|GetLocation) (Transformation|GetActorLocation (.HitActor (Collision|BreakHitResult _array_element))) "TraceTypeQuery2" false _outactors "None"))
            (if (and (== (.HitActor (Collision|BreakHitResult _array_element)) (.HitActor (Collision|BreakHitResult _outhit))) (> (Math|Vector|DotProduct (Transformation|GetActorForwardVector (Pawn|GetControlledPawn (Variables|Default|GetAIControllerRef))) (- (Transformation|GetActorLocation (.HitActor (Collision|BreakHitResult _array_element))) (Variables|Default|GetLocation))) 0.0))
              (Class|BTFunctionLibrary|SetBlackboardValueasObject _targetfollow (.HitActor (Collision|BreakHitResult _outhit)))
              (AI|BehaviorTree|SetBlackboardValueasVector (Variables|Default|GetTargetLocation) (Transformation|GetActorLocation (.HitActor (Collision|BreakHitResult _array_element))))
              (else
                (Class|BTFunctionLibrary|SetBlackboardValueasObject _targetfollow)))))
        (else
          (Class|BTFunctionLibrary|SetBlackboardValueasObject (Variables|Default|GetTargetFollow)))))))