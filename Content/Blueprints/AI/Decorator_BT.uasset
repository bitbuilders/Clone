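; Behavior tree decorator that passes when the AI's pawn is at least a minimum distance from its follow target.
; PerformConditionCheck lazily casts and caches the owning AIControllerFollow_BP on first use.
; It then compares the distance between the controlled pawn and the TargetFollow blackboard actor against DistanceMin.
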(fn PerformConditionCheck
  (params (OwnerActor :type Actor%20Object%20Reference))
  (if (!= (Variables|Default|GetAIControllerRef) 0)
    _
    (else
      (bind _asaicontroller_follow_bp (Utilities|Casting|CastToAIControllerFollow_BP OwnerActor))
      (Variables|Default|SetAIControllerRef _asaicontroller_follow_bp)))
  (return (>= (Math|Vector|VectorLength (- (Transformation|GetActorLocation (Pawn|GetControlledPawn (Variables|Default|GetAIControllerRef))) (Transformation|GetActorLocation (AI|BehaviorTree|GetBlackboardValueasActor (Variables|Default|GetTargetFollow))))) (Variables|Default|GetDistanceMin))))