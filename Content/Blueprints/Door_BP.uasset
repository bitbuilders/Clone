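; Door_BP is an automatic sliding door that opens when something enters its trigger volume and closes when the trigger empties.
; A counter tracks overlapping actors, so the DoorMove timeline reverses only after the last one leaves, following a short delay.
; The timeline lerps the door's relative location from its starting position to DoorEnd.
; Each entry also activates smoke and plays a pressure-release sound at the entering actor.
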(event OnComponentBeginOverlap(Trigger)
  (params (OverlappedComponent :type Primitive%20Component%20Object%20Reference) (OtherActor :type Actor%20Object%20Reference) (OtherComp :type Primitive%20Component%20Object%20Reference) (OtherBodyIndex :type Integer) (bFromSweep :type Boolean) (SweepResult :type Hit%20Result%20Structure%20%28by%20ref%29))
  (Variables|Default|SetPawnsInTrigger (+ (Variables|Default|GetPawnsInTrigger) 1))
  (Components|Activation|Activate (Variables|Default|GetSmoke) false)
  (Audio|PlaySoundatLocation "/Game/Sounds/PressureRelease_Cue.PressureRelease_Cue" (Transformation|GetActorLocation OtherActor) "0, 0, 0" 1.0 1.0 0.0 0 0 0)
  (bind _doorz (Timeline|DoorMove Play)
    (:Update
      (Transformation|SetRelativeLocation (Variables|Default|GetDoor) (Math|Vector|Lerp(Vector) (Variables|Default|GetDoorStart) (Variables|Default|GetDoorEnd) _doorz) false false))))

(event OnComponentEndOverlap(Trigger)
  (params (OverlappedComponent :type Primitive%20Component%20Object%20Reference) (OtherActor :type Actor%20Object%20Reference) (OtherComp :type Primitive%20Component%20Object%20Reference) (OtherBodyIndex :type Integer))
  (Variables|Default|SetPawnsInTrigger (- (Variables|Default|GetPawnsInTrigger) 1))
  (if (< (Variables|Default|GetPawnsInTrigger) 1)
    (Utilities|FlowControl|Delay 0.2)
    (bind _doorz (Timeline|DoorMove Reverse)
      (:Update
        (Transformation|SetRelativeLocation (Variables|Default|GetDoor) (Math|Vector|Lerp(Vector) (Variables|Default|GetDoorStart) (Variables|Default|GetDoorEnd) _doorz) false false)))))

(event EventBeginPlay
  (Variables|Default|SetDoorStart (Variables|/Script/Engine.SceneComponent|GetRelativeLocation (Variables|Default|GetDoor))))

(event Collision|EventActorBeginOverlap
  (params (OtherActor :type Actor%20Object%20Reference)))

(event EventTick
  (params (DeltaSeconds :type Float%20%28single-precision%29)))

(fn ConstructionScript)