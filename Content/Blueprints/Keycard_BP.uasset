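; Keycard pickup that spins in place and increments the first-person character's key count when collected.
; On pawn overlap with its box, it plays a sound, then disables the card mesh's collision and hides it.
; For the player character, it waits briefly, spawns a replacement keycard above one of the first four TargetPoints found in the level, chosen at random, then destroys itself.
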(event OnComponentBeginOverlap(Box)
  (params (OverlappedComponent :type Primitive%20Component%20Object%20Reference) (OtherActor :type Actor%20Object%20Reference) (OtherComp :type Primitive%20Component%20Object%20Reference) (OtherBodyIndex :type Integer) (bFromSweep :type Boolean) (SweepResult :type Hit%20Result%20Structure%20%28by%20ref%29))
  (bind _cartd (Variables|Default|GetCartd))
  (bind _aspawn (Utilities|Casting|CastToPawn OtherActor))
  (Audio|PlaySoundatLocation "/Game/Sounds/CardPickup.CardPickup" (Transformation|GetActorLocation _aspawn) "0, 0, 0" 1.0 1.0 0.0 0 0 0)
  (bind _outactors (Actor|GetAllActorsOfClass "/Script/Engine.TargetPoint"))
  (Collision|SetCollisionEnabled _cartd "NoCollision")
  (Rendering|SetVisibility _cartd false false)
  (bind _asfirst_person_character (Utilities|Casting|CastToFirstPersonCharacter _aspawn))
  (Variables|/Game/FirstPersonBP/Blueprints/FirstPersonCharacter.FirstPersonCharacter_C|SetKeyCount _asfirst_person_character (+ (Variables|/Game/FirstPersonBP/Blueprints/FirstPersonCharacter.FirstPersonCharacter_C|GetKeyCount _asfirst_person_character) 1))
  (Utilities|FlowControl|Delay 3.0)
  (Game|SpawnActorfromClass "Keycard_BP_C" (Math|Conversions|ToTransform(Vector) (+ (Transformation|GetActorLocation (Utilities|Array|Get(acopy) _outactors (Math|Random|RandomIntegerinRange 0 3))) "0, 0,50.000000")) "Undefined" 0 0)
  (Actor|DestroyActor))

(event EventBeginPlay)

(event Collision|EventActorBeginOverlap
  (params (OtherActor :type Actor%20Object%20Reference)))

(event EventTick
  (params (DeltaSeconds :type Float%20%28single-precision%29))
  (Transformation|AddLocalRotation (Variables|Default|GetCartd) "0,1.000000, 0" false false))

(fn ConstructionScript)