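; Game mode that shows the UI widget and keeps the level supplied with AI enemies, raising the enemy cap as time passes.
; A looping timer counts live AICharacter_BP actors and, while below MaxEnemies, spawns one running Logic_BT at a random pick among the first four TargetPoints found.
; Tick accumulates time and increments MaxEnemies whenever EnemyIncreaseTime elapses.
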(event Custom|Respawn
  (bind _outactors (Actor|GetAllActorsOfClass "/Game/Blueprints/AI/AICharacter_BP.AICharacter_BP_C"))
  (if (< (Utilities|Array|Length _outactors) (Variables|Default|GetMaxEnemies))
    (bind _outactors_2 (Actor|GetAllActorsOfClass "/Script/Engine.TargetPoint"))
    (AI|SpawnAIFromClass "/Game/Blueprints/AI/AICharacter_BP.AICharacter_BP_C" "/Game/Blueprints/AI/Logic_BT.Logic_BT" (Transformation|GetActorLocation (Utilities|Array|Get(acopy) _outactors_2 (Math|Random|RandomIntegerinRange 0 3))) "0, 0, 0" false)))

(event EventBeginPlay
  (bind _returnvalue (UserInterface|CreateWidget "/Game/UI.UI_C" (Game|GetPlayerController 0)))
  (UserInterface|Viewport|AddtoViewport _returnvalue 0)
  (Utilities|Time|SetTimerbyEvent (delegate Custom|Respawn) 1.5 true))

(event EventTick
  (params (DeltaSeconds :type Float%20%28single-precision%29))
  (Variables|Default|SetEnemyTime (+ DeltaSeconds (Variables|Default|GetEnemyTime)))
  (if (>= (Variables|Default|GetEnemyTime) (Variables|Default|GetEnemyIncreaseTime))
    (Variables|Default|SetMaxEnemies (+ (Variables|Default|GetMaxEnemies) 1))
    (Variables|Default|SetEnemyTime 0.0)))

(fn ConstructionScript)